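; BP_Camera is an actor in the trailer folder, set up as a view-target camera for a rotating shot.
; A Cast event switches the first-person player controller's TempWidget to shop mode.
; An unconnected chain would, after a delay, call it, blend the view to this actor and lerp its rotation on the MOVE timeline.
; BeginPlay is empty, so nothing here starts the shot, and a location lerp is also unwired.
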(event `Cast`
  (bind _asbp_first_person_player_controller (cast `/Game/FirstPerson/Blueprints/BP_FirstPersonPlayerController` (`GameplayStatics.GetPlayerController` 0)))
  (`/Game/Shop-and-inventory/WBP_TempHUD.Shop Mode` (`/Game/FirstPerson/Blueprints/BP_FirstPersonPlayerController.TempWidget` _asbp_first_person_player_controller)))

(event `self.ReceiveBeginPlay`)

(fn `UserConstructionScript`)