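; BP_TestTrap is a placeholder trap actor that deals fear damage when an actor implementing BPI_Test overlaps its sphere.
; It reads the Trap_1 row of DT_Trap at BeginPlay for terror radius and damage.
; The overlap runs a debug-drawn, zero-length multi-sphere trace at the cube.
; A DoOnce limits processing to the first hit, sending DamageMessage if it implements the interface, then resets.
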(event `self.ReceiveBeginPlay`
  (bind _returnvalue (`|GetDataTableRow` "/Game/DataTables/DT_Trap.DT_Trap" "Trap_1")))

(event `Reset`
  (goto _label :!via `Reset`))

(event `self.Sphere.OnComponentBeginOverlap`
  (params (OverlappedComponent :type "PrimitiveComponent Object Reference") (OtherActor :type "Actor Object Reference") (OtherComp :type "PrimitiveComponent Object Reference") (OtherBodyIndex :type Integer) (bFromSweep :type Boolean) (SweepResult :type "HitResult Structure (by ref)"))
  (bind _returnvalue (`SceneComponent.K2_GetComponentLocation` (`self.Cube`)))
  (if (`KismetSystemLibrary.DoesImplementInterface` OtherActor "/Game/DataTables/BPI_Test.BPI_Test_C")
    (bind _outhits (`KismetSystemLibrary.SphereTraceMulti` :`Start` _returnvalue :`End` _returnvalue :`Radius` (`.TerrorRadius_4_AEA3D46E42A1D59C31437899F2FB6BFB` (break `/Game/DataTables/STR_Trap` (stale `self.ReceiveBeginPlay` _returnvalue))) :`TraceChannel` "TraceTypeQuery2" :`DrawDebugType` "ForDuration"))
    (for _array_element _outhits
      (`/Engine/EditorBlueprintResources/StandardMacros.DoOnce` false :!label _label
        (:`Completed`
          (bind (_bblockinghit _binitialoverlap _time _distance _location _impactpoint _normal _impactnormal _physmat _hitactor) (`GameplayStatics.BreakHitResult` _array_element))
          (`KismetSystemLibrary.PrintString` (`KismetSystemLibrary.GetDisplayName` _hitactor))
          (if (`KismetSystemLibrary.DoesImplementInterface` _hitactor "/Game/DataTables/BPI_Test.BPI_Test_C")
            (message `/Game/DataTables/BPI_Test.Damage` _hitactor (`.FearDamage_5_543BC00D49F70BB46963339A4CE2967C` (break `/Game/DataTables/STR_Trap` (stale `self.ReceiveBeginPlay` _returnvalue))))))))
    (`self.Reset`)))

(fn `UserConstructionScript`)