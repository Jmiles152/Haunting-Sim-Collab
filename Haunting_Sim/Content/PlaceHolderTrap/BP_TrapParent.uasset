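; BP_TrapParent is a placeholder trap, apparently a base class, that sends a damage message to nearby actors when E is pressed.
; E runs a debug-drawn sphere trace at the mesh; a DoOnce, cleared by Reset, lets one hit through to receive zero damage via BPI_Test.
; PlayerInRangeCircle overlaps set IsPlayerInRange, which the trigger never reads.
; The end-overlap interface check has no actor connected.
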(event `Key|E`
  (params (Key :type "Key Structure"))
  (bind _returnvalue (`SceneComponent.K2_GetComponentLocation` (`self.StaticMesh`)))
  (:`Pressed`
    (bind _outhits (`KismetSystemLibrary.SphereTraceMulti` :`Start` _returnvalue :`End` _returnvalue :`TraceChannel` "TraceTypeQuery2" :`DrawDebugType` "ForDuration"))
    (for _array_element _outhits
      (`/Engine/EditorBlueprintResources/StandardMacros.DoOnce` false :!label _label
        (:`Completed`
          (bind (_bblockinghit _binitialoverlap _time _distance _location _impactpoint _normal _impactnormal _physmat _hitactor) (`GameplayStatics.BreakHitResult` _array_element))
          (`KismetSystemLibrary.PrintString` (`KismetSystemLibrary.GetDisplayName` _hitactor))
          (if (`KismetSystemLibrary.DoesImplementInterface` _hitactor "/Game/DataTables/BPI_Test.BPI_Test_C")
            (message `/Game/DataTables/BPI_Test.Damage` _hitactor 0.0)))))))

(event `self.PlayerInRangeCircle.OnComponentBeginOverlap`
  (params (OverlappedComponent :type "PrimitiveComponent Object Reference") (OtherActor :type "Actor Object Reference") (OtherComp :type "PrimitiveComponent Object Reference") (OtherBodyIndex :type Integer) (bFromSweep :type Boolean) (SweepResult :type "HitResult Structure (by ref)"))
  (if (`KismetSystemLibrary.DoesImplementInterface` OtherActor "/Game/DataTables/BPI_Test.BPI_Test_C")
    (set `self.IsPlayerInRange` true)))

(event `Reset`
  (goto _label :!via `Reset`))

(event `self.PlayerInRangeCircle.OnComponentEndOverlap`
  (params (OverlappedComponent :type "PrimitiveComponent Object Reference") (OtherActor :type "Actor Object Reference") (OtherComp :type "PrimitiveComponent Object Reference") (OtherBodyIndex :type Integer))
  (if (`KismetSystemLibrary.DoesImplementInterface` null "/Game/DataTables/BPI_Test.BPI_Test_C")
    (set `self.IsPlayerInRange` false)))

(fn `UserConstructionScript`)