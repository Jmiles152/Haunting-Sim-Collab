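; Placeholder test trap that makes an audible noise and reports it as a "Scare" noise event for AI hearing.
; On BeginPlay it casts the player character to BP_FirstPersonCharacter and binds an event to its JumpScare through BindEventToJumpScare.
; PlayNoise plays the drop sound and reports the noise at the trap's location, with the trap as instigator.
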(event `self.ReceiveBeginPlay`
  (`parent.ReceiveBeginPlay`)
  (bind _asbp_first_person_character (cast `/Game/FirstPerson/Blueprints/BP_FirstPersonCharacter` (`GameplayStatics.GetPlayerCharacter` 0)))
  (add `/Game/FirstPerson/Blueprints/BP_FirstPersonCharacter.JumpScare` _asbp_first_person_character (`|CreateDelegate` :!event `Play Noise`)))

(event `Play Noise`
  (bind _returnvalue (`self.K2_GetActorLocation`))
  (`GameplayStatics.PlaySoundAtLocation` "/Game/Audio/SC_Drop.SC_Drop" _returnvalue (struct) 1.0 1.0 0.0 null null null null)
  (`AISense_Hearing.ReportNoiseEvent` _returnvalue 1.0 self 0.0 "Scare"))

(fn `UserConstructionScript`
  (`parent.UserConstructionScript`))