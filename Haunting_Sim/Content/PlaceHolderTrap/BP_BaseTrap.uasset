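; Base trap actor that scares or lures NPCs when triggered at night, with stats pulled from DT_TrapBackup by row name.
; Triggering plays a sound and sphere-traces the terror radius, notifying BPI_TrapNotify actors.
; If none are found, it briefly becomes a "Scare"-tagged sight stimulus and reports noise to lure AI.
; DoOnce gates and timers handle limited-use rearming or cooldown; TrapEffects is an empty visuals hook, and FixedTrapToggle sets activation by trap class.
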(event Custom|Cooldown
  ;[0.15 0.15 0.15 0.5] Trap rearm + Timer
  (Utilities|Time|SetTimerbyEvent (EventDispatchers|CreateEvent :!event Custom|CooldownSet) (.ReArmTime (Utilities|Struct|BreakSTR_TrapBackup (Variables|Default|GetStats)))))

(event Custom|Play%20Noise
  (bind _returnvalue (Transformation|GetActorLocation))
  ;[0.15 0.15 0.15 0.5] Overlap Trigger
  ;;[0.15 0.15 0.15 0.5] Rearm Check
  (if (.LimitedUse? (Utilities|Struct|BreakSTR_TrapBackup (Variables|Default|GetStats)))
    (Utilities|FlowControl|DoOnce false
      (:Completed
        _))
    (else
      (Utilities|FlowControl|DoOnce false
        (:Completed
          _))))
  (Audio|PlaySoundatLocation "/Game/Audio/Cues/SC_Drop.SC_Drop" _returnvalue "0, 0, 0" 1.0 1.0 0.0 0 0 0 0)
  (bind _outhits (Collision|MultiSphereTraceForObjects _returnvalue _returnvalue (.TerrorRadius (Utilities|Struct|BreakSTR_TrapBackup (Variables|Default|GetStats))) (Utilities|Array|MakeArray "ObjectTypeQuery8") true 0 "None"))
  (for _array_element _outhits
    (if (Utilities|DoesObjectImplementInterface (.HitActor (Collision|BreakHitResult _array_element)) "/Game/DataTables/BPI_TrapNotify.BPI_TrapNotify_C")
      (Class|BPITrapNotify|TerrorRadius(Message) (.HitActor (Collision|BreakHitResult _array_element)) self)
      (Variables|Default|SetInScareRadius? true)))
  (if (Variables|Default|GetInScareRadius?)
    _
    (else
      (CallFunction|Lure)))
  (CallFunction|Resetting))

(event Custom|RearmSet
  (bind _returnvalue (Transformation|GetActorLocation))
  ;[0.15 0.15 0.15 0.5] Overlap Trigger
  ;;[0.15 0.15 0.15 0.5] Rearm Counter
  (Variables|Default|SetArms (+ (Variables|Default|GetArms) 1))
  (Utilities|FlowControl|DoOnce false) ; enters at Reset
)

(event Custom|DayEnd
  (Variables|Default|SetNight? true))

(event Custom|Resetting
  ;[0.15 0.15 0.15 0.5] Comment
  (if (.LimitedUse? (Utilities|Struct|BreakSTR_TrapBackup (Variables|Default|GetStats)))
    (CallFunction|Re-Arm)
    (else
      (CallFunction|Cooldown))))

(event Custom|Lure
  ;[0.15 0.15 0.15 0.5] Luring NPC
  (Utilities|Array|Add (Variables|Actor|GetTags) "Scare")
  (Class|AIPerceptionStimuliSourceComponent|RegisterforSense (Variables|Default|GetAIPerceptionStimuliSource) "/Script/AIModule.AISense_Sight")
  (Utilities|FlowControl|Delay 0.2)
  (Class|AISenseHearing|ReportNoiseEvent (Transformation|GetActorLocation) 1e+01 self 0.0 "Scare")
  (Utilities|FlowControl|Delay 1.0)
  (Utilities|Array|RemoveItem (Variables|Actor|GetTags) "Scare")
  (Class|AIPerceptionStimuliSourceComponent|UnregisterfromSense (Variables|Default|GetAIPerceptionStimuliSource) "/Script/AIModule.AISense_Sight"))

(event Custom|FixedTrapToggle
  (params (DesiredTrapToActivate :type BP%20Base%20Trap%20Class%20Reference) (Activate :type Boolean))
  ;[0.15 0.15 0.15 0.5] W7 Activating fixed traps when one is brought in the shop
  ;;[0.15 0.15 0.15 0.5] Seeing if this trap is the type of trap that needs to be activated, can also be used to deactivate a class of traps
  (bind _returnvalue (Utilities|GetDataTableRow "/Game/DataTables/DT_TrapBackup.DT_TrapBackup" (Variables|Default|GetRow%20Name))
    (:then
      (if (== DesiredTrapToActivate (.Class (Utilities|Struct|BreakSTR_TrapBackup _returnvalue)))
        (Variables|Default|SetFixedTrapActive Activate)))))

(event Custom|CooldownSet
  (bind _returnvalue (Transformation|GetActorLocation))
  ;[0.15 0.15 0.15 0.5] Overlap Trigger
  (Utilities|FlowControl|DoOnce false) ; enters at Reset
)

(event Custom|AttentionRadius
  (bind _cube (Variables|Default|GetCube))
  (bind _returnvalue (Transformation|GetWorldLocation _cube))
  ;[0.15 0.15 0.15 0.5] Do not use, for screenshots and scraping code if necessary
  ;;[0.15 0.15 0.15 0.5] AttentionRadius
  (bind _outhits (Collision|MultiSphereTraceByChannel _returnvalue _returnvalue 0.0 "TraceTypeQuery2" false 0 "ForDuration"))
  (for _array_element _outhits
    (Utilities|FlowControl|DoOnce false
      (:Completed
        (if (Utilities|DoesObjectImplementInterface (.HitActor (Collision|BreakHitResult _array_element)) "/Game/DataTables/BPI_TrapNotify.BPI_TrapNotify_C")
          _))))
  (CallFunction|ResetAttention))

(event Custom|ResetAttention
  ;[0.15 0.15 0.15 0.5] Do not use, for screenshots and scraping code if necessary
  ;;[0.15 0.15 0.15 0.5] AttentionRadius
  (Utilities|FlowControl|DoOnce false) ; enters at Reset
)

(event Custom|KeyActive
  (Variables|Default|SetKeyUsed? true))

(event Custom|ResetTerror
  ;[0.15 0.15 0.15 0.5] Do not use, for screenshots and scraping code if necessary
  ;;[0.15 0.15 0.15 0.5] TerrorRadius
  (Utilities|FlowControl|DoOnce false) ; enters at Reset
)

(event Custom|TrapEffects
  ;[0.15 0.15 0.15 0.5] Trap effects (for visuals)
)

(event Custom|Re-Arm
  (bind _stats (Variables|Default|GetStats))
  (bind (_isauto_ _limiteduse_ _trapcost _terrorradius _attentionradius _feardamage _trapuses _rearmtime) (Utilities|Struct|BreakSTR_TrapBackup _stats))
  ;[0.15 0.15 0.15 0.5] Trap rearm + Timer
  (if (not (>= (Variables|Default|GetArms) _trapuses))
    (Utilities|Time|SetTimerbyEvent (EventDispatchers|CreateEvent :!event Custom|RearmSet) _rearmtime)))

(event Custom|NightEnd
  (Variables|Default|SetNight? false))

(event EventBeginPlay
  ;[0.15 0.15 0.15 0.5] Player and GameMode refs
  (Utilities|Casting|CastToBP_FirstPersonCharacter (Game|GetPlayerCharacter 0))
  (bind _asbp_first_person_game_mode (Utilities|Casting|CastToBP_FirstPersonGameMode (Game|GetGameMode)))
  ;[0.15 0.15 0.15 0.5] Pulls data from data table
  (bind _returnvalue (Utilities|GetDataTableRow "/Game/DataTables/DT_TrapBackup.DT_TrapBackup" (Variables|Default|GetRow%20Name))
    (:then
      (EventDispatchers|BindEventtoStartOfNightTrigger _asbp_first_person_game_mode (delegate Custom|DayEnd))
      (EventDispatchers|BindEventtoStartOfDayTrigger _asbp_first_person_game_mode (delegate Custom|NightEnd))
      (Variables|Default|SetStats _returnvalue))))

(event EventTrigger
  ;[0.15 0.15 0.15 0.5] Interact triggers trap
  (if (Variables|Default|GetNight?)
    (CallFunction|PlayNoise)
    (CallFunction|TrapEffects)))

(fn ConstructionScript)

(fn GetRowName
  (return (Variables|Default|GetRow%20Name)))

(fn GetTrapData
  (bind _stats (Variables|Default|GetStats))
  (bind (_isauto_ _limiteduse_ _trapcost _terrorradius _attentionradius _feardamage _trapuses _rearmtime _pointreward _displayname _class _previewmesh _traptype _score _moneyreward) (Utilities|Struct|BreakSTR_TrapBackup _stats))
  (return (Math|Float|Truncate _feardamage) (Math|Conversions|ToFloat(Integer) _score) (Math|Conversions|ToFloat(Integer) _moneyreward)))