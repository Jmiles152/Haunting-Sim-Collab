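; BP_Fixed_Fridge is a trap Blueprint that acts as a proxy for a BP_NewFridge actor in the level.
; On BeginPlay it caches the actor returned by GetActorOfClass and prints its name.
; Trigger defers to the parent, while TrapEffects forwards to the cached fridge's TrapEffects without calling the parent version or checking that the reference is valid.
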(event `self.ReceiveBeginPlay`
  (`parent.ReceiveBeginPlay`)
  (bind _returnvalue (`GameplayStatics.GetActorOfClass` "/Game/Art/Props/Kitchen/Fridge/BP_NewFridge.BP_NewFridge_C"))
  (bind _output_get (set `self.FridgeRef` _returnvalue))
  (`KismetSystemLibrary.PrintString` (`KismetSystemLibrary.GetDisplayName` _output_get)))

(event `self.Trigger`
  (`parent.Trigger`))

(event `self.TrapEffects`
  (`/Game/Art/Props/Kitchen/Fridge/BP_NewFridge.TrapEffects` (`self.FridgeRef`)))

(fn `UserConstructionScript`
  (`parent.UserConstructionScript`))