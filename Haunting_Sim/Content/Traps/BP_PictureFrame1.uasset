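; BP_PictureFrame1 is a picture frame trap that plays a sound and rattles crooked when its TrapEffects event fires.
; The Turn timeline lerps the mesh's relative roll from level toward a random angle in either direction.
; The random value is re-rolled on every timeline update, so the frame jitters instead of turning smoothly.
; After the timeline finishes, a delay holds the final tilt before resetting the rotation to zero.
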(event `self.TrapEffects`
  (bind _staticmesh (`self.StaticMesh`))
  (`GameplayStatics.PlaySoundAtLocation` null (`self.K2_GetActorLocation`) (struct) 1.0 1.0 0.0 null null null null)
  (bind (_direction _alpha) (`Timeline|Turn`)
    (:`Update`
      (`SceneComponent.K2_SetRelativeRotation` _staticmesh (`KismetMathLibrary.MakeRotator` (`KismetMathLibrary.Lerp` 0.0 (`KismetMathLibrary.RandomFloatInRange` -50.0 50.0) _alpha)) false false))
    (:`Finished`
      (`KismetSystemLibrary.Delay` 5.0)
      (`SceneComponent.K2_SetRelativeRotation` :`self` _staticmesh))))

(fn `UserConstructionScript`
  (`parent.UserConstructionScript`))