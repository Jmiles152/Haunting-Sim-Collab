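; BP_Mug is a trap child Blueprint in which a mug pops and leaves a decal.
; TrapEffects plays the Mug sound and starts a timer that fires PopTime shortly before two seconds pass.
; PopTime briefly shows Pop alongside the Decal, then hides Pop and the mug.
; The decal then fades out and destroys the actor, while Trigger only forwards to the parent.
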(event `self.Trigger`
  (`parent.Trigger`))

(event `self.TrapEffects`
  (`GameplayStatics.PlaySoundAtLocation` "/Game/Shop-and-inventory/ThingsToRelocate/Mug.Mug" (`self.K2_GetActorLocation`) (struct) 1.0 1.0 0.0 null null null null)
  (`KismetSystemLibrary.K2_SetTimerDelegate` (delegate `PopTime`) 1.82))

(event `PopTime`
  (bind _pop (`self.Pop`))
  (`SceneComponent.SetVisibility` _pop true false)
  (`SceneComponent.SetVisibility` (`self.Decal`) true false)
  (`KismetSystemLibrary.Delay` 0.1)
  (`SceneComponent.SetVisibility` _pop false false)
  (`SceneComponent.SetVisibility` (`self.Mug`) false false)
  (`DecalComponent.SetFadeOut` (`self.Decal`) 1.0 1.0 true))

(fn `UserConstructionScript`
  (`parent.UserConstructionScript`))