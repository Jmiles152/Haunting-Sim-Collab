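; BP_Globe is a trap prop whose globe mesh spins when TrapEffects fires, then eases off.
; The Rotate timeline adds a fixed local rotation to StaticMesh1 on each update, then calls Finish.
; Finish plays the Slowing timeline, whose Alpha blends that per-update step toward zero.
; Rotation is applied per timeline update without delta-time scaling, so spin speed follows frame rate.
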(event `self.TrapEffects`
  (`Timeline|Rotate`
    (:`Update`
      (`SceneComponent.K2_AddLocalRotation` (`self.StaticMesh1`) (struct :`Yaw` 10.0) false false))
    (:`Finished`
      (`self.Finish`))))

(event `Finish`
  (bind (_direction _alpha) (`Timeline|Slowing`)
    (:`Update`
      (`SceneComponent.K2_AddLocalRotation` (`self.StaticMesh1`) (`KismetMathLibrary.RLerp` (struct :`Yaw` 10.0) (struct) _alpha) false false))))

(fn `UserConstructionScript`
  (`parent.UserConstructionScript`))