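; BP_Book is a book trap actor that moves vertically when lured.
; It overrides the Lure event, calls the parent's version, then records the current Z height and restarts the Float timeline.
; Each timeline update offsets the actor from that height by the scaled track value, leaving X and Y unchanged.
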(event `self.Lure`
  (bind (_returnvalue_x _returnvalue_y _returnvalue_z) (`KismetMathLibrary.BreakVector` (`self.K2_GetActorLocation`)))
  (bind (_returnvalue_x_2 _returnvalue_y_2) (`KismetMathLibrary.BreakVector` (`self.K2_GetActorLocation`)))
  (`parent.Lure`)
  (set `self.Z` _returnvalue_z)
  (bind (_direction _newtrack_0) (`Timeline|Float` :!via `PlayFromStart`)
    (:`Update`
      (`self.K2_SetActorLocation` (`KismetMathLibrary.MakeVector` _returnvalue_x_2 _returnvalue_y_2 (+ (* _newtrack_0 15.0) (`self.Z`)))))))

(fn `UserConstructionScript`
  (`parent.UserConstructionScript`))