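; BP_Plates is a trap Blueprint that makes a pair of plates clatter when its effects fire.
; TrapEffects restarts the Clatter timeline, whose movement track lerps Plate1 and Plate2 along relative Z over different height ranges.
; An event track on the same timeline plays the Clink sound at the actor's location, while Trigger defers to the parent class.
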(event `self.Trigger`
  (`parent.Trigger`))

(event `self.TrapEffects`
  (bind (_direction _platemovement) (`Timeline|Clatter` :!via `PlayFromStart`)
    (:`Update`
      (`SceneComponent.K2_SetRelativeLocation` (`self.Plate2`) (`KismetMathLibrary.MakeVector` 0.0 0.0 (`KismetMathLibrary.Lerp` 6.0 46.0 _platemovement)) false false)
      (`SceneComponent.K2_SetRelativeLocation` (`self.Plate1`) (`KismetMathLibrary.MakeVector` 0.0 0.0 (`KismetMathLibrary.Lerp` 4.0 30.0 _platemovement)) false false))
    (:`SoundCue`
      (`GameplayStatics.PlaySoundAtLocation` "/Game/Shop-and-inventory/ThingsToRelocate/Clink.Clink" (`self.K2_GetActorLocation`) (struct) 1.0 1.0 0.0 null null null null))))

(fn `UserConstructionScript`
  (`parent.UserConstructionScript`))