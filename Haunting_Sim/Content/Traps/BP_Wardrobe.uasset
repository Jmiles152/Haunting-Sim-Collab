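; Wardrobe trap actor whose two hinged doors swing open when Trigger is called.
; Right and Left each use a FlipFlop to play or reverse a timeline that lerps its hinge from the rotation cached at BeginPlay.
; When a timeline finishes, a short delay re-calls its event, flipping that door between open and closed.
; World rotations are cached but applied as relative rotations.
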(event `self.ReceiveBeginPlay`
  (`parent.ReceiveBeginPlay`)
  (set `self.RightRote` (`SceneComponent.K2_GetComponentRotation` (`self.RightHinge`)))
  (set `self.LeftRote` (`SceneComponent.K2_GetComponentRotation` (`self.LeftHinge`))))

(event `self.Trigger`
  (`self.Right`)
  (`self.Left`))

(event `Right`
  (`/Engine/EditorBlueprintResources/StandardMacros.FlipFlop`
    (:`A`
      (bind (_direction _alpha) (`Timeline|RightOpen` :!via `PlayFromStart` :!label _label)
        (:`Update`
          (`SceneComponent.K2_SetRelativeRotation` (`self.RightHinge`) (`KismetMathLibrary.RLerp` (`self.RightRote`) (`KismetMathLibrary.ComposeRotators` (`self.RightRote`) (struct :`Yaw` -70.0)) _alpha true) false false))
        (:`Finished`
          (`KismetSystemLibrary.Delay` 3.0)
          (`self.Right`))))
    (:`B`
      (goto _label :!via `ReverseFromEnd`))))

(event `Left`
  (`/Engine/EditorBlueprintResources/StandardMacros.FlipFlop`
    (:`A`
      (bind (_direction _alpha) (`Timeline|LeftOpen` :!via `PlayFromStart` :!label _label_2)
        (:`Update`
          (`SceneComponent.K2_SetRelativeRotation` (`self.LeftHinge`) (`KismetMathLibrary.RLerp` (`self.LeftRote`) (`KismetMathLibrary.ComposeRotators` (`self.LeftRote`) (struct :`Yaw` 130.0)) _alpha true) false false))
        (:`Finished`
          (`KismetSystemLibrary.Delay` 3.0)
          (`self.Left`))))
    (:`B`
      (goto _label_2 :!via `ReverseFromEnd`))))

(fn `UserConstructionScript`
  (`parent.UserConstructionScript`))