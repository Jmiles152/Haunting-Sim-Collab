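; BP_Fridge is a fridge Blueprint in the SmartObject folder that supplies food actors to whoever takes from it.
; Its SpawnFood function spawns a random class from the supplied list, has the given attachment actor pick it up, and returns the spawned actor.
; The event graph and construction script add no logic of their own, so SpawnFood runs only when called.
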(fn `Spawn Food`
  (params (`Attachment Actor` :type "/Game/AI/BP_NPC Object Reference") (`Actors To Spawn` :type "Array of Actor Class Reference"))
  (returns (Spawned :type "Actor Object Reference"))
  (bind _returnvalue (`|SpawnActorFromClass` (`KismetArrayLibrary.Array_Random` `Actors To Spawn`) (`KismetMathLibrary.MakeTransform` (0.0 0.0 0.0)) "Undefined" "MultiplyWithRoot" null null))
  (`/Game/AI/BP_NPC.Pick Up Object` `Attachment Actor` _returnvalue)
  (return _returnvalue))

(fn `UserConstructionScript`
  (`parent.UserConstructionScript`))