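; NPC Blueprint that reacts to scares it sees or hears through AI Perception, losing Sanity that a looping timer gradually restores.
; Seen scare actors lose their tag; heard scares from currently visible sources only unregister that source's stimuli.
; Other scares trigger OnJumpScare, which stops movement and sends an Interruption event with noise data to the StateTree.
; Helpers claim random nearby Smart Objects by tag and attach picked-up objects to the hand.
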(event `self.AIPerception.OnTargetPerceptionUpdated`
  (params (Actor :type "Actor Object Reference") (Stimulus :type "AIStimulus Structure"))
  (bind _returnvalue (`AIPerceptionSystem.GetSenseClassForStimulus` Stimulus))
  (if (== _returnvalue "/Script/AIModule.AISense_Sight")
    (`self.Saw Something` Actor Stimulus)
    (else
      (`self.Heard Something` Actor Stimulus))))

(event `Restore Sanity`
  (if (< (`self.Sanity`) 10)
    (`/Engine/EditorBlueprintResources/StandardMacros.IncrementInt` (`self.Sanity`))))

(event `self.ReceiveBeginPlay`
  (`KismetSystemLibrary.K2_SetTimerDelegate` (delegate `Restore Sanity`) 10.0 true))

(event `Pick Up Object`
  (params (`Object To Pick Up` :type "Actor Object Reference"))
  (`self.K2_AttachToComponent` `Object To Pick Up` (`self.Mesh`) "ik_hand_rSocket" "KeepRelative" "KeepRelative" "KeepRelative" true)
  (`self.K2_SetActorRelativeTransform` `Object To Pick Up` (`KismetMathLibrary.MakeTransform` (0.0 0.0 0.0)) false false))

(event `OnJumpScare`
  (params (Instigator :type "Actor Object Reference"))
  (`/Engine/EditorBlueprintResources/StandardMacros.DecrementInt` (`self.Sanity`)
    (:`  `
      (if (== Instigator (`self.Last Trap Sensed`))
        _
        (else
          _))
      (bind _returnvalue (`BlueprintInstancedStructLibrary.MakeInstancedStruct` (make `/Game/AI/F_NoiseData` Instigator)))
      (`self.JumpScare`)
      (`self.Cleanup Behaviour`)
      (`Controller.StopMovement` (`AIBlueprintHelperLibrary.GetAIController` self))
      (`StateTreeComponent.SendStateTreeEvent` (`self.GetComponentByClass` (`AIBlueprintHelperLibrary.GetAIController` self) "/Script/GameplayStateTreeModule.StateTreeAIComponent") (make `StateTreeEvent` (struct :`TagName` "Interruption") _returnvalue "External")))))

(fn `Find Random Smart Object With Tag`
  (params (Tags :type "GameplayTagContainer Structure" :default (struct :`GameplayTags` (struct :`(TagName` "Action.Sit")))))
  (returns (`Smart Object Claim Handle` :type "SmartObjectClaimHandle Structure") (Found :type Boolean))
  (bind (_outresults _returnvalue) (`SmartObjectSubsystem.FindSmartObjects_BP` (subsystem `SmartObjectSubsystem`) (make `SmartObjectRequest` (`KismetMathLibrary.MakeBoxWithOrigin` (`self.K2_GetActorLocation`) (2000.0 2000.0 2000.0)) (make `SmartObjectRequestFilter` Tags)) self))
  (if _returnvalue
    (bind _returnvalue_2 (`SmartObjectBlueprintFunctionLibrary.MarkSmartObjectSlotAsClaimed` (`.SlotHandle` (break `SmartObjectRequestResult` (`KismetArrayLibrary.Array_Random` _outresults))) (`AIBlueprintHelperLibrary.GetAIController` self)))
    (return _returnvalue_2 true)
    (else
      (return (struct) false))))

(fn `Heard Something`
  (params (Instigator :type "Actor Object Reference") (Stimulus :type "AIStimulus Structure"))
  (locals (`Seeing While Hearing` :type Boolean) (Inst :type "Actor Object Reference"))
  (set `local.Inst` Instigator)
  (if (== (`.Tag` (break `AIStimulus` Stimulus)) "Scare")
    (for _array_element (`AIPerceptionComponent.GetCurrentlyPerceivedActors` (`self.AIPerception`) "/Script/AIModule.AISense_Sight")
      (if (== _array_element (`local.Inst`))
        (`AIPerceptionStimuliSourceComponent.UnregisterFromPerceptionSystem` (`self.GetComponentByClass` _array_element "/Script/AIModule.AIPerceptionStimuliSourceComponent"))
        (return)))
    (`KismetSystemLibrary.PrintString` "What was that?" true true (struct :`R` 1.0 :`G` 0.00488 :`B` 0.910851 :`A` 1.0))
    (`self.OnJumpScare` (`local.Inst`))))

(fn `Saw Something`
  (params (Instigator :type "Actor Object Reference") (Stimulus :type "AIStimulus Structure"))
  (if (`self.ActorHasTag` Instigator "Scare")
    (`KismetArrayLibrary.Array_RemoveItem` (`Actor.Tags` Instigator) "Scare")
    (`KismetSystemLibrary.PrintString` "Nah I saw that shit" true true (struct :`R` 1.0 :`B` 0.722365 :`A` 1.0))
    (`self.OnJumpScare` Instigator)))

(fn `UserConstructionScript`)