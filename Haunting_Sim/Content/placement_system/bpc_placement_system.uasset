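; Player component for placing and picking up buildable traps, with a build mode toggled by input.
; Each tick in build mode, a camera line trace positions a collisionless preview mesh, created through a resettable DoOnce and yawed left by a looping timer.
; Placing spawns the active inventory slot's class and fires TrapPlaced; destroying returns "buildable"-tagged actors to inventory if space allows.
; Right rotation, scroll selection and build-list refresh are disconnected or empty.
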(event `self.ReceiveBeginPlay`
  ; cast to player, as well as set up the databace of building materials, to scroll through
  (bind _asbp_first_person_character (cast `/Game/FirstPerson/Blueprints/BP_FirstPersonCharacter` (`self.GetOwner`)))
  (set `self.player bp` _asbp_first_person_character)
  (set `self.First Person Camera` (`/Game/FirstPerson/Blueprints/BP_FirstPersonCharacter.FirstPersonCamera` _asbp_first_person_character))
  ;[0.15 0.1235 0 0.5] The items available to build must be updated when the inventory contents changes
  (bind _returnvalue (`GameplayStatics.GetActorOfClass` "/Game/Shop-and-inventory/BP_InventoryManager.BP_InventoryManager_C"))
  (bind _output_get (set `self.Inventory_Ref` _returnvalue))
  (add `/Game/Shop-and-inventory/BP_InventoryManager.UpdateInventoryContents` _output_get (delegate `RefreshBuildOptions`))
  (add `/Game/Shop-and-inventory/BP_InventoryManager.ChangeSlot` _output_get (delegate `SlotChanged`)))

(event `RefreshBuildOptions`)

(event `self.ReceiveTick`
  (params (DeltaSeconds :type "Float (single-precision)"))
  ; createing the preview mesh
  (if (`self.in_build_mode`)
    (`self.preview_loop`)))

(event `preview_loop`
  (bind (_returnvalue_location _returnvalue_rotation) (`KismetMathLibrary.BreakTransform` (`SceneComponent.K2_GetComponentToWorld` (`self.First Person Camera`))))
  (bind _returnvalue (`KismetMathLibrary.GetForwardVector` _returnvalue_rotation))
  ; main setup behind scenes, getting the world tansform and telling the blueprint what to do
  (bind _outhit (`KismetSystemLibrary.LineTraceSingle` _returnvalue_location (+ _returnvalue (* _returnvalue (`self.preview_distance`))) "TraceTypeQuery1"))
  (if true
    (`|ExecutionSequence`
      (:`then_0`
        (`/Engine/EditorBlueprintResources/StandardMacros.DoOnce` false :!label _label
          (:`Completed`
            (bind _returnvalue_2 (`|AddComponentByClass` (`self.player bp`) "/Script/Engine.StaticMeshComponent" false (`self.build  preview Transform`)))
            (bind _output_get (set `self.preview_mesh` _returnvalue_2))
            (`StaticMeshComponent.SetStaticMesh` _output_get (`.PreviewMesh_39_E3B0B0A7455E79BE50412C94F3D03FF5` (break `/Game/DataTables/STR_TrapBackup` (`|GetArrayItem` (`self.dt_build_parts`) (`self.buildable index`)))))
            (`PrimitiveComponent.SetMaterial` (`self.preview_mesh`) 0 "/Game/placement_system/materials/m_build_preview.m_build_preview")
            (`PrimitiveComponent.SetCollisionEnabled` (`self.preview_mesh`) "NoCollision"))))
      (:`then_1`
        (bind _output_get_2 (set `self.build  preview Transform` (`KismetMathLibrary.MakeTransform` (`.Location` (`GameplayStatics.BreakHitResult` _outhit)) (`self.build_preview_rotate_left`))))
        (`SceneComponent.K2_SetWorldTransform` (`self.preview_mesh`) _output_get_2 false false)))))

(event `reset_build_mode`
  ; main setup behind scenes, getting the world tansform and telling the blueprint what to do
  (goto _label :!via `Reset`))

(event `EnhancedInput|/Game/placement_system/imputs/imputs/ia_build`
  (params (ActionValue :type Boolean) (ElapsedSeconds :type "Float (double-precision)") (TriggeredSeconds :type "Float (double-precision)") (InputAction :type "InputAction Object Reference" :default "/Game/placement_system/imputs/imputs/ia_build.ia_build"))
  ; setting up build mode, to display
  (:`Started`
    (if (not (`self.in_build_mode`))
      (set `self.in_build_mode` true)
      (else
        (set `self.in_build_mode` false :!label _label_2)
        (bind _preview_mesh (`self.preview_mesh`)
          (:`then`
            (`StaticMeshComponent.SetStaticMesh` _preview_mesh null)
            (set `self.preview_mesh` null)
            (`self.reset_build_mode`)
            ;[0.15 0.1107 0 0.5] Added for UI updates
            (`self.ToggleBuildMode`))
          (:`else`))))))

(event `stop_build_mode`
  ; setting up build mode, to display
  (goto _label_2))

(event `EnhancedInput|/Game/placement_system/imputs/imputs/ia_place_build`
  (params (ActionValue :type Boolean) (ElapsedSeconds :type "Float (double-precision)") (TriggeredSeconds :type "Float (double-precision)") (InputAction :type "InputAction Object Reference" :default "/Game/placement_system/imputs/imputs/ia_place_build.ia_place_build"))
  ; spawning objects
  (:`Started`
    (if (`self.in_build_mode`)
      (`|SpawnActorFromClass` (`.Class_45_2C6C9015401BC5C8D61F35A30AC56375` (break `/Game/DataTables/STR_TrapBackup` (`|GetArrayItem` (`self.dt_build_parts`) (`self.buildable index`)))) (`self.build  preview Transform`) "AlwaysSpawn" "MultiplyWithRoot" null null)
      ;;[0.15 0.1142 0 0.5] For removing from inventory
      (`self.TrapPlaced`)
      (`self.stop_build_mode`))))

(event `Key|MouseScrollDown`
  (params (Key :type "Key Structure"))
  ; scroll through placement options (disconnected due to functionality being moved to inventory manager)
)

(event `EnhancedInput|/Game/placement_system/imputs/imputs/ia_rotate_left`
  (params (ActionValue :type Boolean) (ElapsedSeconds :type "Float (double-precision)") (TriggeredSeconds :type "Float (double-precision)") (InputAction :type "InputAction Object Reference" :default "/Game/placement_system/imputs/imputs/ia_rotate_left.ia_rotate_left"))
  ; rotate the object left
  (:`Started`
    (bind _returnvalue (`KismetSystemLibrary.K2_SetTimerDelegate` (delegate `rotate_preview_left`) 0.1 true))
    (set `self.build_rotate_preview-loop_left` _returnvalue))
  (:`Completed`
    (`KismetSystemLibrary.K2_ClearAndInvalidateTimerHandle` (`self.build_rotate_preview-loop_left`))
    (set `self.build_rotate_preview-loop_left` (struct))))

(event `rotate_preview_left`
  (bind (_build__preview_transform_location _build__preview_transform_rotation) (`KismetMathLibrary.BreakTransform` (`self.build  preview Transform`)))
  ; rotate the object left
  (set `self.build_preview_rotate_left` (`KismetMathLibrary.ComposeRotators` _build__preview_transform_rotation (`KismetMathLibrary.MakeRotator` 0.0 0.0 (`self.rotate_value_z_left`)))))

(event `SlotChanged`
  ; scroll through placement options (disconnected due to functionality being moved to inventory manager)
  ;;[0.15 0.119 0 0.5] Now based off inventory slots
  (set `self.buildable index` (`/Game/Shop-and-inventory/BP_InventoryManager.ActiveSlot` (`self.Inventory_Ref`)))
  (bind _preview_mesh (`self.preview_mesh`)
    (:`then`
      (`StaticMeshComponent.SetStaticMesh` _preview_mesh null)
      (set `self.preview_mesh` null)
      (`self.reset_build_mode`))
    (:`else`)))

(event `Key|MouseScrollUp`
  (params (Key :type "Key Structure"))
  ; scroll through placement options (disconnected due to functionality being moved to inventory manager)
)

(event `EnhancedInput|/Game/placement_system/imputs/imputs/ia_rotate_right`
  (params (ActionValue :type Boolean) (ElapsedSeconds :type "Float (double-precision)") (TriggeredSeconds :type "Float (double-precision)") (InputAction :type "InputAction Object Reference" :default "/Game/placement_system/imputs/imputs/ia_rotate_right.ia_rotate_right"))
  ; tried ti get the rotate to work the other way
)

(event `EnhancedInput|/Game/placement_system/imputs/imputs/ia_destroy`
  (params (ActionValue :type Boolean) (ElapsedSeconds :type "Float (double-precision)") (TriggeredSeconds :type "Float (double-precision)") (InputAction :type "InputAction Object Reference" :default "/Game/placement_system/imputs/imputs/ia_destroy.ia_destroy"))
  (bind (_returnvalue_location _returnvalue_rotation) (`KismetMathLibrary.BreakTransform` (`SceneComponent.K2_GetComponentToWorld` (`self.First Person Camera`))))
  (bind _returnvalue (`KismetMathLibrary.GetForwardVector` _returnvalue_rotation))
  (:`Started`
    ; destroys placed objects
    ;;[0.15 0.1019 0 0.5] Traps can only be picked back up if there is room in the inventory, not sure if demolishing traps should eb a thing?
    (bind _spaceavailable (`/Game/Shop-and-inventory/BP_InventoryManager.InventoryHasSpace` (`self.Inventory_Ref`)))
    (if _spaceavailable
      (bind (_outhit _returnvalue_2) (`KismetSystemLibrary.LineTraceSingle` _returnvalue_location (+ _returnvalue (* _returnvalue (`self.preview_distance`))) "TraceTypeQuery1"))
      (if _returnvalue_2
        (bind (_bblockinghit _binitialoverlap _time _distance _location _impactpoint _normal _impactnormal _physmat _hitactor) (`GameplayStatics.BreakHitResult` _outhit))
        ;; Adding destroyed items back into the inventory
        (if (`Actor.ActorHasTag` _hitactor "buildable")
          (`/Game/Shop-and-inventory/BP_InventoryManager.AddToInventory` (`self.Inventory_Ref`) (`BlueprintMapLibrary.Map_Find` (`self.ActorToRowNameMap`) (`GameplayStatics.GetObjectClass` _hitactor)))
          (`Actor.K2_DestroyActor` _hitactor))))))

(event `rotate_preview_right`
  ; tried ti get the rotate to work the other way
)