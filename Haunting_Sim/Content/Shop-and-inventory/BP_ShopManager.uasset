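; BP_ShopManager is a trap shop actor that switches the player to UI mode and rerolls its stock on overlap, restoring gameplay mode on exit.
; Stock is random row names from DT_TrapBackup, filled at BeginPlay if empty.
; Purchases go through BP_InventoryManager, deducting cost and removing the item from stock.
; A parallel Buyability array tracks currency and inventory space, refreshed before CallShopOptionsUpdated announces stock changes.
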(event `self.ReceiveActorBeginOverlap`
  (params (OtherActor :type "Actor Object Reference"))
  (`/Game/FirstPerson/Blueprints/BP_FirstPersonPlayerController.UIMode` (cast `/Game/FirstPerson/Blueprints/BP_FirstPersonPlayerController` (`GameplayStatics.GetPlayerController` 0) :!pure true))
  (`self.ShopRandomise` (`self.DefaultQuantityAvailable`)))

(event `self.ReceiveBeginPlay`
  ; Set up on start
  (bind _returnvalue (`GameplayStatics.GetActorOfClass` "/Game/Shop-and-inventory/BP_InventoryManager.BP_InventoryManager_C"))
  (set `self.InventoryManagerRef` _returnvalue)
  (if (`KismetArrayLibrary.Array_IsEmpty` (`self.AvailableItems`))
    (`self.ShopRandomise` (`self.DefaultQuantityAvailable`)) ; If the shop is empty new items will be added
    (else
      (`self.CheckBuyability`))))

(event `self.ReceiveActorEndOverlap`
  (params (OtherActor :type "Actor Object Reference"))
  (`/Game/FirstPerson/Blueprints/BP_FirstPersonPlayerController.GameplayMode` (cast `/Game/FirstPerson/Blueprints/BP_FirstPersonPlayerController` (`GameplayStatics.GetPlayerController` 0) :!pure true)))

(event `ShopRandomise`
  (params (NewQuantityAvailable :type Integer))
  ; Randomise the items available in the shop
  (`KismetArrayLibrary.Array_Clear` (`self.AvailableItems`))
  (bind _outrownames (`DataTableFunctionLibrary.GetDataTableRowNames` "/Game/DataTables/DT_TrapBackup.DT_TrapBackup"))
  (for _ (range 1 (+ (`KismetMathLibrary.SelectInt` (`self.DefaultQuantityAvailable`) NewQuantityAvailable (== NewQuantityAvailable 0)) 1))
    (`KismetArrayLibrary.Array_Add` (`self.AvailableItems`) (`KismetArrayLibrary.Array_Random` _outrownames)))
  (`self.CheckBuyability`) ; Will always run after new items are added
  (`self.ShopOptionsUpdated`))

(event `ItemBought`
  (params (Index :type Integer))
  (bind _inventorymanagerref (`self.InventoryManagerRef`))
  (bind _availableitems (`self.AvailableItems`))
  (bind _output (`|GetArrayItem` _availableitems Index))
  ; Player buys an item
  (`KismetArrayLibrary.Array_Add` (`self.SellHistory`) _output)
  (bind _returnvalue (`|GetDataTableRow` "/Game/DataTables/DT_TrapBackup.DT_TrapBackup" _output)
    (:`then`
      (`/Game/Shop-and-inventory/BP_InventoryManager.AddToInventory` _inventorymanagerref _output)
      (`/Game/Shop-and-inventory/BP_InventoryManager.RemoveCurrency` _inventorymanagerref (`.BaseCost_26_F687BD6C434EE30EC8D89082BF6C36F1` (break `/Game/DataTables/STR_TrapBackup` _returnvalue)))
      (`KismetArrayLibrary.Array_Remove` _availableitems Index)
      (`self.CheckBuyability`) ; Will always run after new items are added
      (`self.ShopOptionsUpdated`))))

(event `CheckInventorySpace`
  ; Must run before cost check to remain accurate
  (bind _spaceavailable (`/Game/Shop-and-inventory/BP_InventoryManager.InventoryHasSpace` (`self.InventoryManagerRef`)))
  (set `self.PlayerInventoryUnfilled` _spaceavailable))

(event `CheckBuyability`
  ; Checking if the player can buy anything based on the cost and available inventory space
  (`self.CheckInventorySpace`)
  (`KismetArrayLibrary.Array_Clear` (`self.Buyability`))
  (for _array_element (`self.AvailableItems`)
    (bind _returnvalue (`|GetDataTableRow` "/Game/DataTables/DT_TrapBackup.DT_TrapBackup" _array_element)
      (:`then`
        (`KismetArrayLibrary.Array_Add` (`self.Buyability`) (and (>= (`/Game/Shop-and-inventory/BP_InventoryManager.Currency` (`self.InventoryManagerRef`)) (`.BaseCost_26_F687BD6C434EE30EC8D89082BF6C36F1` (break `/Game/DataTables/STR_TrapBackup` _returnvalue))) (`self.PlayerInventoryUnfilled`)))))))

(fn `UserConstructionScript`)