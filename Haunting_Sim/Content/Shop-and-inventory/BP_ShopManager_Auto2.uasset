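; Shop manager actor that sells randomly picked traps from DT_TrapBackup through the player's inventory manager.
; Actor overlap switches to UI mode and rerolls stock, while sphere overlap adds the shop widget.
; Per-item buyability follows currency and inventory space, refreshed after rerolls and purchases.
; Purchases are recorded under key 0 for Refund, which removes the item but calls RemoveCurrency again rather than crediting the cost.
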(event `self.ReceiveActorBeginOverlap`
  (params (OtherActor :type "Actor Object Reference"))
  (`/Game/FirstPerson/Blueprints/BP_FirstPersonPlayerController.UIMode` (cast `/Game/FirstPerson/Blueprints/BP_FirstPersonPlayerController` (`GameplayStatics.GetPlayerController` 0) :!pure true))
  (`self.ShopRandomise` (`self.DefaultQuantityAvailable`)))

(event `self.ReceiveBeginPlay`
  ; Set up on start
  (bind _returnvalue (`GameplayStatics.GetActorOfClass` "/Game/Shop-and-inventory/BP_InventoryManager_New.BP_InventoryManager_New_C"))
  (set `self.InventoryManagerRef` _returnvalue)
  (if (`KismetArrayLibrary.Array_IsEmpty` (`self.AvailableItems`))
    (`self.ShopRandomise` (`self.DefaultQuantityAvailable`)) ; If the shop is empty new items will be added
    (else
      (`self.CheckBuyability`))))

(event `self.ReceiveActorEndOverlap`
  (params (OtherActor :type "Actor Object Reference"))
  (`/Game/FirstPerson/Blueprints/BP_FirstPersonPlayerController.GameplayMode` (cast `/Game/FirstPerson/Blueprints/BP_FirstPersonPlayerController` (`GameplayStatics.GetPlayerController` 0) :!pure true)))

(event `ShopRandomise`
  (params (NewQuantityAvailable :type Integer))
  ; Randomise the items available in the shop
  (`KismetArrayLibrary.Array_Clear` (`self.AvailableItems`))
  (bind _outrownames (`DataTableFunctionLibrary.GetDataTableRowNames` "/Game/DataTables/DT_TrapBackup.DT_TrapBackup"))
  (for _ (range 1 (+ (`KismetMathLibrary.SelectInt` (`self.DefaultQuantityAvailable`) NewQuantityAvailable (== NewQuantityAvailable 0)) 1))
    (`KismetArrayLibrary.Array_Add` (`self.AvailableItems`) (`KismetArrayLibrary.Array_Random` _outrownames)))
  (`self.CheckBuyability`) ; Will always run after new items are added
  (`self.ShopOptionsUpdated`))

(event `self.Sphere.OnComponentBeginOverlap`
  (params (OverlappedComponent :type "PrimitiveComponent Object Reference") (OtherActor :type "Actor Object Reference") (OtherComp :type "PrimitiveComponent Object Reference") (OtherBodyIndex :type Integer) (bFromSweep :type Boolean) (SweepResult :type "HitResult Structure (by ref)"))
  (bind _returnvalue (`|CreateWidget` "/Game/UI/ShopUI/WBP_shopui.WBP_shopui_C" null null null))
  (`UserWidget.AddToViewport` _returnvalue 0))

(event `self.Sphere.OnComponentEndOverlap`
  (params (OverlappedComponent :type "PrimitiveComponent Object Reference") (OtherActor :type "Actor Object Reference") (OtherComp :type "PrimitiveComponent Object Reference") (OtherBodyIndex :type Integer)))

(event `ItemBought`
  (params (Index :type Integer))
  (bind _inventorymanagerref (`self.InventoryManagerRef`))
  (bind _output (`|GetArrayItem` (`self.AvailableItems`) Index))
  ; Player buys an item
  (bind _returnvalue (`|GetDataTableRow` "/Game/DataTables/DT_TrapBackup.DT_TrapBackup" _output)
    (:`then`
      (bind _destinationindex (`/Game/Shop-and-inventory/BP_InventoryManager_New.AddToInventory` _inventorymanagerref _output))
      (bind (_isauto_ _limiteduse_ _trapcost) (break `/Game/DataTables/Structs/STR_TrapBackup` _returnvalue))
      (`BlueprintMapLibrary.Map_Add` (`self.SellHistory`) 0 (make `/Game/Shop-and-inventory/STR_Sale` _trapcost _destinationindex))
      (`/Game/Shop-and-inventory/BP_InventoryManager_New.RemoveCurrency` _inventorymanagerref _trapcost)
      (`self.CheckBuyability`) ; Will always run after new items are added
      (`self.ShopOptionsUpdated`))))

(event `CheckInventorySpace`
  ; Must run before cost check to remain accurate
  (bind _spaceavailable (`/Game/Shop-and-inventory/BP_InventoryManager_New.InventoryHasSpace` (`self.InventoryManagerRef`)))
  (set `self.PlayerInventoryUnfilled` _spaceavailable))

(event `CheckBuyability`
  ; Checking if the player can buy anything based on the cost and available inventory space
  (`self.CheckInventorySpace`)
  (`KismetArrayLibrary.Array_Clear` (`self.Buyability`))
  (for _array_element (`self.AvailableItems`)
    (bind _returnvalue (`|GetDataTableRow` "/Game/DataTables/DT_TrapBackup.DT_TrapBackup" _array_element)
      (:`then`
        (`KismetArrayLibrary.Array_Add` (`self.Buyability`) (and (>= (`/Game/Shop-and-inventory/BP_InventoryManager_New.Currency` (`self.InventoryManagerRef`)) (`.TrapCost_26_462208314237E7B785F3FDA9E6C0C148` (break `/Game/DataTables/Structs/STR_TrapBackup` _returnvalue))) (`self.PlayerInventoryUnfilled`)))))))

(event `ShopClosed`
  (`BlueprintMapLibrary.Map_Clear` (`self.SellHistory`))
  (`self.ShopClosedDown`))

(event `Refund`
  (params (ShopEntryToRefund :type Integer))
  (bind _inventorymanagerref (`self.InventoryManagerRef`))
  (bind (_cost _invindex) (break `/Game/Shop-and-inventory/STR_Sale` (`BlueprintMapLibrary.Map_Find` (`self.SellHistory`) ShopEntryToRefund)))
  (`/Game/Shop-and-inventory/BP_InventoryManager_New.RemoveIndexFromInventory` _inventorymanagerref _invindex)
  (`/Game/Shop-and-inventory/BP_InventoryManager_New.RemoveCurrency` _inventorymanagerref _cost))

(fn `UserConstructionScript`)