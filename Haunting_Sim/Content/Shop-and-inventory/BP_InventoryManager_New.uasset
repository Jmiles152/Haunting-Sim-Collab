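; Inventory manager actor that tracks the player's currency and trap slots, with "None" marking an empty slot.
; Scrolling skips empty slots and wraps via a rollover map, while dispatchers announce slot, content and most currency changes.
; UseTrap looks up the active item in DT_TrapBackup, then spawns Ability traps at the player or toggles the placement system for Free Place traps, whose placed event clears the slot.
; CheckUsability is unfinished.
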(event `self.ReceiveBeginPlay`
  (bind _returnvalue (`GameplayStatics.GetActorOfClass` "/Game/Shop-and-inventory/BP_ShopManager.BP_ShopManager_C"))
  (set `self.ShopRef` _returnvalue)
  (bind _returnvalue_2 (`GameplayStatics.GetActorOfClass` "/Game/FirstPerson/Blueprints/BP_FirstPersonCharacter.BP_FirstPersonCharacter_C"))
  (bind _output_get (set `self.PlacementRef` (`/Game/FirstPerson/Blueprints/BP_FirstPersonCharacter.bpc_placement_system` _returnvalue_2)))
  (add `/Game/placement_system/bpc_placement_system.TrapPlaced` _output_get (delegate `RemoveCurrentInventory`))
  (`KismetSystemLibrary.Delay` 1.0))

(event `RemoveCurrency`
  (params (Amount :type Integer))
  ; Remove an amount of currency
  (set `self.Currency` (- (`self.Currency`) Amount))
  (`self.UpdateInventoryContents` :!label _label))

(event `AddCurrency`
  (params (Amount :type Integer))
  (set `self.Currency` (+ Amount (`self.Currency`)))
  (goto _label))

(event `RemoveCurrentInventory`
  ; Remove an item from the inventory
  (`|VariableSetRef` (`|GetArrayItem` (`self.Items in inventory`) (`self.ActiveSlot`))) ; Empty
  (`self.UpdateInventoryContents` :!label _label_2))

(event `RemoveIndexFromInventory`
  (params (IndexToRemove :type Integer))
  ; Remove an item from the inventory
  (`|VariableSetRef` (`|GetArrayItem` (`self.Items in inventory`) IndexToRemove)) ; Empty
  (goto _label_2))

(event `ScrollInventorySlot`
  (params (Input :type "Float (double-precision)"))
  ; Inventory slot scrolling, skips empty slots.
  (for _index (range 1 9)
    (bind _returnvalue (+ (`self.ActiveSlot`) (* _index (`KismetMathLibrary.FClamp` Input -1.0))))
    (bind _value (`BlueprintMapLibrary.Map_Find` (`self.InventorySlotRollOverMap`) _returnvalue))
    (bind _returnvalue_2 (and (<= _returnvalue 7) (>= _returnvalue 0)))
    (if (not (== "None" (`|GetArrayItem` (`self.Items in inventory`) (`KismetMathLibrary.SelectInt` _returnvalue _value _returnvalue_2))))
      (bind _output_get (set `self.ActiveSlot` (`KismetMathLibrary.SelectInt` _returnvalue _value _returnvalue_2)))
      (`KismetSystemLibrary.PrintString` (`KismetStringLibrary.Conv_NameToString` (`|GetArrayItem` (`self.Items in inventory`) _output_get)))
      (break)))
  (`self.ChangeSlot`))

(event `ChangeInventorySlot`
  (params (NewSlot :type Integer))
  (set `self.ActiveSlot` NewSlot)
  (`self.ChangeSlot`))

(event `UseTrap`
  (bind _returnvalue (`|GetDataTableRow` "/Game/DataTables/DT_TrapBackup.DT_TrapBackup" (`|GetArrayItem` (`self.Items in inventory`) (`self.ActiveSlot`)))
    (:`then`
      (bind (_isauto_ _limiteduse_ _trapcost _terrorradius _attentionradius _feardamage _trapuses _rearmtime _pointreward _displayname _class _previewmesh _traptype) (break `/Game/DataTables/Structs/STR_TrapBackup` _returnvalue))
      (switch `/Game/DataTables/E_TrapTypes` _traptype
        (:`NewEnumerator0`
          (`|SpawnActorFromClass` _class (`self.GetTransform` (`GameplayStatics.GetPlayerPawn` 0)) "Undefined" "MultiplyWithRoot" null null)
          (`self.RemoveCurrentInventory`))
        (:`NewEnumerator1`
          (`/Game/placement_system/bpc_placement_system.BuildToggle` (`self.PlacementRef`)))))))

(event `self.ReceiveActorBeginOverlap`
  (params (OtherActor :type "Actor Object Reference"))
  ; Refresh the temp UI
  (`self.UpdateInventoryContents`))

(event `/Game/PlaceHolderTrap/BPI_Payout.Change Score`
  (params (Score :type Integer) (Money :type Integer))
  ;[0.4072 0.03955 0.3005 0.502] Adds money to internal currency variable on trap successful scare, shouldn't conflict with anything - kaydon
  (set `self.Currency` (+ (`self.Currency`) Money)))

(event `CheckUsability`
  (`KismetArrayLibrary.Array_Clear` (`self.Usability`))
  (for _array_element (`self.Items in inventory`)
    (bind _returnvalue (`|GetDataTableRow` "/Game/DataTables/DT_TrapBackup.DT_TrapBackup" _array_element))))

(fn `AddToInventory`
  (params (NewItem :type Name))
  (returns (DestinationIndex :type Integer))
  (locals (LocalDestinationIndex :type Integer))
  (bind _items_in_inventory (`self.Items in inventory`))
  ; Find an empty slot to add new item
  (bind _output_get (set `local.LocalDestinationIndex` (`KismetArrayLibrary.Array_Find` _items_in_inventory)))
  (`|VariableSetRef` (`|GetArrayItem` _items_in_inventory _output_get) NewItem)
  (`self.UpdateInventoryContents`)
  (return (`local.LocalDestinationIndex`)))

(fn `InventoryHasSpace`
  (returns (SpaceAvailable :type Boolean) (AvailableIndex :type Integer))
  (for (_array_element _array_index) (`self.Items in inventory`)
    (if (== _array_element "None")
      (`|ExecutionSequence`
        (:`then_0`
          (break))
        (:`then_1`
          (return true _array_index)))))
  (return false 0))

(fn `UserConstructionScript`)