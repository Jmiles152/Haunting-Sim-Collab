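; BP_Mug is a kitchen prop Blueprint for a mug with selectable looks.
; Its Construction Script reads the Variation value and sets one of four mug materials on the first slot of the SMMug mesh.
; Any other Variation value leaves the material unchanged, and the event graph holds only disabled placeholder events, so it has no runtime logic.
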(fn `UserConstructionScript`
  (bind _variation (`self.Variation`))
  (bind _sm_mug (`self.SM_Mug`))
  (if (== _variation 1)
    (`PrimitiveComponent.SetMaterial` _sm_mug 0 "/Game/Art/Props/Kitchen/Mug/materials/M_Mug1.M_Mug1")
    (elif (== _variation 2)
      (`PrimitiveComponent.SetMaterial` _sm_mug 0 "/Game/Art/Props/Kitchen/Mug/materials/M_Mug2.M_Mug2")
      (elif (== _variation 3)
        (`PrimitiveComponent.SetMaterial` _sm_mug 0 "/Game/Art/Props/Kitchen/Mug/materials/M_Mug3.M_Mug3")
        (elif (== _variation 4)
          (`PrimitiveComponent.SetMaterial` _sm_mug 0 "/Game/Art/Props/Kitchen/Mug/materials/M_Mug4.M_Mug4"))))))