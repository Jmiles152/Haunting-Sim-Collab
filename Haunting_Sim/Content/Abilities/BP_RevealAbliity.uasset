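; BP_RevealAbliity is a short-lived reveal ability actor that fires on spawn and destroys itself after a one-second timer.
; Activation adds the WBP_GhostReveal widget to the viewport and emits a "Scare"-tagged hearing noise with itself as instigator.
; The "Scare" actor tag and hearing stimulus registration exist only around that noise report, being removed immediately afterward in the same call.
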(event `self.ReceiveBeginPlay`
  (`parent.ReceiveBeginPlay`)
  (`self.ActivateAbility`)
  (`KismetSystemLibrary.K2_SetTimerDelegate` (delegate `Destroy`) 1.0))

(event `Destroy`
  (`self.K2_DestroyActor`))

(fn `ActivateAbility`
  (`parent.ActivateAbility`)
  (bind _returnvalue (`|CreateWidget` "/Game/Abilities/WBP_GhostReveal.WBP_GhostReveal_C"))
  (`UserWidget.AddToViewport` _returnvalue 0)
  (`KismetArrayLibrary.Array_Add` (`self.Tags`) "Scare")
  (`AIPerceptionStimuliSourceComponent.RegisterForSense` (`self.AIPerceptionStimuliSource`) "/Script/AIModule.AISense_Hearing")
  (`AISense_Hearing.ReportNoiseEvent` (0.0 0.0 0.0) 1.0 self 0.0 "Scare")
  (`KismetArrayLibrary.Array_RemoveItem` (`self.Tags`) "Scare")
  (`AIPerceptionStimuliSourceComponent.UnregisterFromSense` (`self.AIPerceptionStimuliSource`) "/Script/AIModule.AISense_Hearing"))

(fn `UserConstructionScript`
  (`parent.UserConstructionScript`))