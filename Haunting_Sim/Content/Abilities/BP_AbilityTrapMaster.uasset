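; Base trap ability actor that, on spawn, detects NPCs around the first-person player and currently only prints their names.
; BeginPlay caches the player, then AffectNPCInRadius runs a sphere trace of AbilityRadius at the player's location, not the trap's.
; Hits whose class is exactly BP_NPC, excluding subclasses, are collected into NPCsInRadius and returned.
; ActivateAbility is an empty stub, and no effect is applied to the NPCs.
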(event `self.ReceiveBeginPlay`
  (`KismetSystemLibrary.PrintString` "ABILITY TRAP SPAWNED")
  (`parent.ReceiveBeginPlay`)
  (bind _returnvalue (`GameplayStatics.GetActorOfClass` "/Game/FirstPerson/Blueprints/BP_FirstPersonCharacter.BP_FirstPersonCharacter_C"))
  (set `self.PlayerRef` _returnvalue)
  ; TerrorRadiusCalculations
  (bind _affectednpcs (`self.AffectNPCInRadius`))
  (for _array_element _affectednpcs
    (`KismetSystemLibrary.PrintString` (`KismetSystemLibrary.GetDisplayName` _array_element))))

(fn `ActivateAbility`)

(fn `AffectNPCInRadius`
  (returns (AffectedNPCs :type "Array of /Game/AI/BP_NPC Object Reference"))
  (locals (NPCsInRadius :type "Array of /Game/AI/BP_NPC Object Reference"))
  (bind _returnvalue (`self.K2_GetActorLocation` (`self.PlayerRef`)))
  (bind _outhits (`KismetSystemLibrary.SphereTraceMultiForObjects` _returnvalue _returnvalue (`self.AbilityRadius`) (`|MakeArray` "ObjectTypeQuery8" :!type "EObjectTypeQuery Enum")))
  (for _array_element _outhits
    (bind (_bblockinghit _binitialoverlap _time _distance _location _impactpoint _normal _impactnormal _physmat _hitactor) (`GameplayStatics.BreakHitResult` _array_element))
    (if (== (`GameplayStatics.GetObjectClass` _hitactor) "/Game/AI/BP_NPC.BP_NPC_C")
      (`KismetArrayLibrary.Array_Add` (`local.NPCsInRadius`) (cast `/Game/AI/BP_NPC` _hitactor :!pure true))))
  (return (`local.NPCsInRadius`)))

(fn `UserConstructionScript`
  (`parent.UserConstructionScript`))