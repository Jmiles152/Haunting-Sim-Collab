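; BP_WhisperAbility is an ability actor that plays a whisper sound from the player's position.
; On BeginPlay it calls ActivateAbility, which runs the parent logic, plays the whisper at the player's location and adds a "Scare" tag to itself.
; Nodes for hearing-sense registration, noise reporting and tag cleanup are present but unwired, so this Blueprint never reports the whisper to AI perception or removes the tag.
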(event `self.ReceiveBeginPlay`
  (`parent.ReceiveBeginPlay`)
  (`self.ActivateAbility`))

(fn `ActivateAbility`
  (`parent.ActivateAbility`)
  (`GameplayStatics.PlaySoundAtLocation` "/Game/Abilities/Whisper-I_mHere.Whisper-I_mHere" (`self.K2_GetActorLocation` (`self.PlayerRef`)) (struct) 1.0 1.0 0.0 null null null null)
  (`KismetArrayLibrary.Array_Add` (`self.Tags`) "Scare"))

(fn `UserConstructionScript`
  (`parent.UserConstructionScript`))